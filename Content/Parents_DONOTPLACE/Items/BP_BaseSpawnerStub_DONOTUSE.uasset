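; Parent Blueprint stub for item spawners, handling the editor-visible label and icon of a gun.
; Its construction script writes the gun name to a text component.
; It then wraps each valid material on the GunIcon component in a dynamic material instance, feeding GunTexture into the "GunIcon" texture parameter.
; No spawning logic appears in this graph.
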(fn ConstructionScript
  (Rendering|Components|TextRender|SetText (Variables|Default|GetGunName) (Utilities|Text|ToText(String) (Variables|Gun|GetGun%20Name)))
  (for _index (range 0 (Rendering|Material|GetNumMaterials (Variables|Default|GetGunIcon)))
    (Utilities|IsValid (Rendering|Material|GetMaterial (Variables|Default|GetGunIcon) _index)
      (:Is%20Valid
        (bind _returnvalue (Rendering|Material|CreateDynamicMaterialInstance (Rendering|Material|GetMaterial (Variables|Default|GetGunIcon) _index) "None" "None" :!class /Script/Engine.KismetMaterialLibrary))
        (Rendering|Material|SetTextureParameterValue _returnvalue "GunIcon" (Variables|Gun|GetGunTexture))
        (Rendering|Material|SetMaterial (Variables|Default|GetGunIcon) _index _returnvalue)))))