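; A team-tagged player start for Portal Wars, with editor visuals showing which team spawns there.
; The construction script sizes the capsule and labels a text component with the team enum name.
; It looks up the team's colour in a map and applies it to the text, a dynamic floor material's Colour parameter, and the arrow.
; It has no runtime logic.
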(event EventBeginPlay)

(event EventTick
  (params (DeltaSeconds :type Float%20%28single-precision%29)))

(fn ConstructionScript
  (bind _teamtext (Variables|Default|GetTeamText))
  (bind _teamcolours (Variables|Default|GetTeamColours))
  (bind _team (Variables|Default|GetTeam))
  (bind _floor (Variables|Default|GetFloor))
  (bind _value (Utilities|Map|Find _teamcolours _team))
  (Components|Capsule|SetCapsuleSize (Variables|Collision|GetCapsuleComponent) 1.2e+02 5e+01 true)
  (Rendering|Components|TextRender|SetText _teamtext (Utilities|Text|FormatText "Team {Team}" (Utilities|String|EnumtoString (Variables|Default|GetTeam))))
  (Rendering|Components|TextRender|SetTextRenderColor _teamtext (.Value (Utilities|Map|Find (Variables|Default|GetTeamColours) (Variables|Default|GetTeam))))
  (bind _returnvalue (Rendering|Material|CreateDynamicMaterialInstance _floor 0 (Rendering|Material|GetMaterial _floor 0) "None" :!class /Script/Engine.PrimitiveComponent))
  (Rendering|Material|SetVectorParameterValue _returnvalue "Colour" (Math|Conversions|ToLinearColor(Color) _value) :!class /Script/Engine.MaterialInstanceDynamic)
  (bind _arrowcomponent (Variables|Default|GetArrowComponent)
    (:then
      (Variables|/Script/Engine.ArrowComponent|SetArrowColor _arrowcomponent _value))
    (:else)))